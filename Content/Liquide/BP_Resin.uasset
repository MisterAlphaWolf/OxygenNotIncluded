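; BP_Resin is a resin actor that probes its surroundings for neighboring dynamic objects, apparently still in a debug stage.
; Each tick it turns its text label toward the player camera, then fires four short object traces from its Box along the forward and up axes, both ways.
; The hit actors are only printed to screen with the actor's name, and the traces draw debug lines; nothing else reacts to them.
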(event Custom|Linetrace
  (bind _outhit (|LinetraceRight_2))
  (bind _outhit_2 (|LinetraceLeft_2))
  (bind _outhit_3 (|LinetraceUp_2))
  (bind _outhit_4 (|LinetraceDown_2))
  (Development|PrintText (Utilities|Text|FormatText "Actor Hit Left linetrace : {A} 
Actor Hit Right linetrace : {B} 
Actor Hit Up linetrace : {C} 
Actor Hit Down linetrace : {D} 
In Actor : {E}" (.HitActor (Collision|BreakHitResult _outhit_2)) (.HitActor (Collision|BreakHitResult _outhit)) (.HitActor (Collision|BreakHitResult _outhit_3)) (.HitActor (Collision|BreakHitResult _outhit_4)) (Utilities|GetDisplayName self)) true true "(R=0.000000,G=0.660000,B=1.000000,A=1.000000)" 0.0))

(event EventTick
  (params (DeltaSeconds :type Float%20%28single-precision%29))
  (Transformation|SetWorldRotation (Variables|Default|GetTextRender) (Math|Rotator|FindLookatRotation (Transformation|GetWorldLocation (Variables|Default|GetTextRender)) (Transformation|GetActorLocation (Game|GetPlayerCameraManager 0))) false false)
  (CallFunction|Linetrace))

(fn ConstructionScript)