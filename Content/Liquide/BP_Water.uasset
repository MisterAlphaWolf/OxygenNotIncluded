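; Water block actor, apparently an unfinished prototype of grid-like liquid flow that currently only moves along +X.
; Each Tick turns its text toward the camera and runs debug line traces at corners and midpoints, storing hits in misleadingly named "Empty" flags.
; CheckRight makes swept moves until all three right-side traces hit, then clears its timer; CheckLitre destroys the actor without volume.
; One-second looping timers are periodically re-armed; the down timer is unwired.
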(event Custom|CheckAround
  (bind (_lefttopempty _uptopempty) (CallFunction|LineTraceTopLeft))
  (Variables|Booléen|SetLeft%20Top%20Empty _lefttopempty)
  (Variables|Booléen|SetUp%20Top%20Empty _uptopempty)
  (bind (_righttopempty _uprighttopempty) (CallFunction|LineTraceTopRight))
  (Variables|Bool|SetRight%20Top%20Empty _righttopempty)
  (Variables|Booléen|SetUp%20Right%20Top%20Empty _uprighttopempty)
  (bind (_downleftempty _downleftdownempty) (CallFunction|LineTraceDownLeft))
  (Variables|Booléen|SetDown%20Left%20Empty _downleftempty)
  (Variables|Booléen|SetDown%20Left%20Down%20Empty _downleftdownempty)
  (bind (_downrightempty _downrightdownempty) (CallFunction|LineTraceDownRight))
  (Variables|Booléen|SetDown%20Right%20Empty _downrightempty)
  (Variables|Booléen|SetDown%20Right%20Down%20Empty _downrightdownempty)
  (bind (_topmidempty _downmidempty) (CallFunction|LineTraceUpandDown))
  (Variables|Booléen|SetTop%20Mid%20Empty _topmidempty)
  (Variables|Booléen|SetDown%20Mid%20Empty _downmidempty)
  (bind (_leftmid _rightmid) (CallFunction|LineTraceLeftandRight))
  (Variables|Booléen|SetLeft%20Mid _leftmid)
  (Variables|Booléen|SetRight%20Mid _rightmid))

(event Custom|CheckLitre
  (if (> (Variables|float|GetLitre) 0.0)
    (Development|PrintString "sup a 0L" true true "(R=0.000000,G=0.660000,B=1.000000,A=1.000000)" 0.1)
    (else
      (Actor|DestroyActor))))

(event Custom|CheckRight
  (bind _returnvalue (Transformation|GetActorLocation))
  (if (Math|Boolean|ORBoolean (not (Variables|Booléen|GetDown%20Right%20Empty)) (not (Variables|Booléen|GetRight%20Mid)) (not (Variables|Bool|GetRight%20Top%20Empty)))
    (bind _returnvalue_2 (Transformation|SetActorLocation (Math|Interpolation|VInterptoConstant _returnvalue (+ _returnvalue "100.000000,0.000000,0.000000") (Utilities|Time|GetWorldDeltaSeconds) 5e+02) true false))
    (Development|PrintText (Utilities|Text|ToText(Boolean) _returnvalue_2) true true "(R=1.000000,G=0.000000,B=0.064941,A=1.000000)")
    (else
      (Utilities|Time|ClearandInvalidateTimerbyHandle (Variables|Handle|GetRightHandle)))))

(event Custom|ReloadTimer
  (Utilities|Time|SetTimerbyEvent (EventDispatchers|CreateEvent :!event Custom|CheckLitre) 1.0 true true)
  (bind _returnvalue (Utilities|Time|SetTimerbyEvent (EventDispatchers|CreateEvent :!event Custom|CheckRight) 1.0 true true))
  (Variables|Handle|SetRightHandle _returnvalue)
  (Utilities|Time|SetTimerbyEvent (delegate Custom|ReloadTimer) 1e+01 false true))

(event EventTick
  (params (DeltaSeconds :type Float%20%28single-precision%29))
  (Transformation|SetWorldRotation (Variables|Default|GetTextRender) (Math|Rotator|FindLookatRotation (Transformation|GetWorldLocation (Variables|Default|GetTextRender)) (Transformation|GetActorLocation (Game|GetPlayerCameraManager 0))) false false)
  (CallFunction|CheckAround))

(event EventBeginPlay
  (Utilities|Time|SetTimerbyEvent (EventDispatchers|CreateEvent :!event Custom|CheckLitre) 1.0 true true)
  (bind _returnvalue (Utilities|Time|SetTimerbyEvent (EventDispatchers|CreateEvent :!event Custom|CheckRight) 1.0 true true))
  (Variables|Handle|SetRightHandle _returnvalue)
  (Utilities|Time|SetTimerbyEvent (delegate Custom|ReloadTimer) 1e+01 false true))

(fn ConstructionScript)

(fn LineTraceTopLeft
  (bind _topleft (Variables|Default|GetTopLeft))
  (bind _topleft_2 (Variables|Default|GetTopLeft))
  (bind _returnvalue (Transformation|GetWorldLocation _topleft))
  (bind _returnvalue_2 (Transformation|GetWorldLocation _topleft_2))
  (bind _returnvalue_3 (Collision|LineTraceForObjects _returnvalue_2 (+ _returnvalue_2 (* (Math|Vector|GetForwardVector _topleft_2) 2.0)) (Utilities|Array|MakeArray "ObjectTypeQuery1" "ObjectTypeQuery2") false 0 "ForDuration"))
  (bind _returnvalue_4 (Collision|LineTraceForObjects _returnvalue (+ _returnvalue (* (Math|Vector|GetUpVector _topleft) 2.0)) (Utilities|Array|MakeArray "ObjectTypeQuery1" "ObjectTypeQuery2") false 0 "ForDuration"))
  (return _returnvalue_3 _returnvalue_4))

(fn LineTraceTopRight
  (bind _topright (Variables|Default|GetTopRight))
  (bind _topright_2 (Variables|Default|GetTopRight))
  (bind _returnvalue (Transformation|GetWorldLocation _topright))
  (bind _returnvalue_2 (Transformation|GetWorldLocation _topright_2))
  (bind _returnvalue_3 (Collision|LineTraceForObjects _returnvalue_2 (+ _returnvalue_2 (* (Math|Vector|GetForwardVector _topright_2) -2.0)) (Utilities|Array|MakeArray "ObjectTypeQuery1" "ObjectTypeQuery2") false 0 "ForDuration"))
  (bind _returnvalue_4 (Collision|LineTraceForObjects _returnvalue (+ _returnvalue (* (Math|Vector|GetUpVector _topright) 2.0)) (Utilities|Array|MakeArray "ObjectTypeQuery1" "ObjectTypeQuery2") false 0 "ForDuration"))
  (return _returnvalue_3 _returnvalue_4))

(fn LineTraceDownLeft
  (bind _downleft (Variables|Default|GetDownLeft))
  (bind _downleft_2 (Variables|Default|GetDownLeft))
  (bind _returnvalue (Transformation|GetWorldLocation _downleft))
  (bind _returnvalue_2 (Transformation|GetWorldLocation _downleft_2))
  (bind _returnvalue_3 (Collision|LineTraceForObjects _returnvalue_2 (+ _returnvalue_2 (* (Math|Vector|GetForwardVector _downleft_2) 2.0)) (Utilities|Array|MakeArray "ObjectTypeQuery1" "ObjectTypeQuery2") false 0 "ForDuration"))
  (bind _returnvalue_4 (Collision|LineTraceForObjects _returnvalue (+ _returnvalue (* (Math|Vector|GetUpVector _downleft) -2.0)) (Utilities|Array|MakeArray "ObjectTypeQuery1" "ObjectTypeQuery2") false 0 "ForDuration"))
  (return _returnvalue_3 _returnvalue_4))

(fn LineTraceDownRight
  (bind _downright (Variables|Default|GetDownRight))
  (bind _downright_2 (Variables|Default|GetDownRight))
  (bind _returnvalue (Transformation|GetWorldLocation _downright))
  (bind _returnvalue_2 (Transformation|GetWorldLocation _downright_2))
  (bind _returnvalue_3 (Collision|LineTraceForObjects _returnvalue_2 (+ _returnvalue_2 (* (Math|Vector|GetForwardVector _downright_2) -2.0)) (Utilities|Array|MakeArray "ObjectTypeQuery1" "ObjectTypeQuery2") false 0 "ForDuration"))
  (bind _returnvalue_4 (Collision|LineTraceForObjects _returnvalue (+ _returnvalue (* (Math|Vector|GetUpVector _downright) -2.0)) (Utilities|Array|MakeArray "ObjectTypeQuery1" "ObjectTypeQuery2") false 0 "ForDuration"))
  (return _returnvalue_3 _returnvalue_4))

(fn LineTraceUpandDown
  (bind _downmid (Variables|Default|GetDownMid))
  (bind _topmid (Variables|Default|GetTopMid))
  (bind _returnvalue (Transformation|GetWorldLocation _downmid))
  (bind _returnvalue_2 (Transformation|GetWorldLocation _topmid))
  (bind _returnvalue_3 (Collision|LineTraceForObjects _returnvalue_2 (+ _returnvalue_2 (* (Math|Vector|GetUpVector _topmid) -56.0)) (Utilities|Array|MakeArray "ObjectTypeQuery1" "ObjectTypeQuery2") false 0 "ForDuration"))
  (bind _returnvalue_4 (Collision|LineTraceForObjects _returnvalue (+ _returnvalue (* (Math|Vector|GetUpVector _downmid) 56.0)) (Utilities|Array|MakeArray "ObjectTypeQuery1" "ObjectTypeQuery2") false 0 "ForDuration"))
  (return _returnvalue_3 _returnvalue_4))

(fn LineTraceLeftandRight
  (bind _midright (Variables|Default|GetMidRight))
  (bind _midleft (Variables|Default|GetMidLeft))
  (bind _returnvalue (Transformation|GetWorldLocation _midright))
  (bind _returnvalue_2 (Transformation|GetWorldLocation _midleft))
  (bind _returnvalue_3 (Collision|LineTraceForObjects _returnvalue_2 (+ _returnvalue_2 (* (Math|Vector|GetForwardVector _midleft) -56.0)) (Utilities|Array|MakeArray "ObjectTypeQuery1" "ObjectTypeQuery2") false 0 "ForDuration"))
  (bind _returnvalue_4 (Collision|LineTraceForObjects _returnvalue (+ _returnvalue (* (Math|Vector|GetForwardVector _midright) 56.0)) (Utilities|Array|MakeArray "ObjectTypeQuery1" "ObjectTypeQuery2") false 0 "ForDuration"))
  (return _returnvalue_3 _returnvalue_4))